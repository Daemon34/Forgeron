(event Custom|Preview%20Loop
  (bind _camera (Variables|Default|GetCamera))
  (bind _returnvalue (Transformation|GetWorldTransform _camera))
  (bind (_outhit _returnvalue_2) (Collision|LineTraceByChannel (.location _returnvalue) (+ (.location _returnvalue) (* (Math|Vector|GetForwardVector (.rotation _returnvalue)) 8e+03)) "TraceTypeQuery1" false 0 "None"))
  (if _returnvalue_2
    (Utilities|FlowControl|Sequence
      (:then_0
        (Utilities|FlowControl|DoOnce false
          (:Completed
            (bind _returnvalue_3 (Game|AddComponentbyClass (Variables|Default|GetPlayer%20BP) "/Script/Engine.StaticMeshComponent" false (Variables|Default|GetBuild%20Preview%20Transform)))
            (bind _output_get (Variables|Default|SetPreview%20Mesh _returnvalue_3))
            (Components|StaticMesh|SetStaticMesh _output_get "/Game/3D_Assets/Anvil/Anvil.Anvil")
            (Rendering|Material|SetMaterial (Variables|Default|GetPreview%20Mesh) 0 "/Game/M_BuildingPreview.M_BuildingPreview"))))
      (:then_1
        (bind _output_get_2 (Variables|Default|SetBuild%20Preview%20Transform (Math|Transform|MakeTransform (.Location (Collision|BreakHitResult _outhit)) "0, 0, 0" "1.000000,1.000000,1.000000")))
        (Transformation|SetWorldTransform (Variables|Default|GetPreview%20Mesh) _output_get_2 false false)))))

(event Custom|Reset%20Build%20Mode
  (Utilities|FlowControl|DoOnce false) ; enters at Reset
)

(event Input|EnhancedActionEvents|EnhancedInputActionIA_Build
  (params (ActionValue :type Boolean) (ElapsedSeconds :type Float%20%28double-precision%29) (TriggeredSeconds :type Float%20%28double-precision%29) (InputAction :type Input%20Action%20Object%20Reference :default "/Game/ThirdPerson/Input/Actions/IA_Build.IA_Build"))
  (bind _player_mesh (Variables|Default|GetPlayer%20Mesh))
  (:Started
    (Utilities|FlowControl|FlipFlop
      (:A
        (Variables|Default|SetInBuildMode true)
        (Rendering|SetVisibility _player_mesh false false))
      (:B
        (Variables|Default|SetInBuildMode false)
        (Rendering|SetVisibility _player_mesh true false)
        (Components|StaticMesh|SetStaticMesh (Variables|Default|GetPreview%20Mesh) 0)
        (Variables|Default|SetPreview%20Mesh 0)
        (CallFunction|ResetBuildMode)))))

(event EventBeginPlay
  (bind _asbp_third_person_character (Utilities|Casting|CastToBP_ThirdPersonCharacter (Components|GetOwner)))
  (Variables|Default|SetPlayer%20BP _asbp_third_person_character)
  (Variables|Default|SetCamera (Variables|/Script/Forgeron.ForgeronCharacter|GetFollowCamera _asbp_third_person_character))
  (Variables|Default|SetPlayer%20Mesh (Variables|/Script/Engine.Character|GetMesh _asbp_third_person_character)))

(event EventTick
  (params (DeltaSeconds :type Float%20%28single-precision%29))
  (if (Variables|Default|GetInBuildMode)
    (CallFunction|PreviewLoop)))